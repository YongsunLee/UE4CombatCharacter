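; BP_BaseRole is a player-controlled samurai character with camera-relative movement, running, defending, equipping, attacks and directional dodges.
; A timeline ramps walk speed for running, defending cancels the run, and Tick enables orient-to-movement only while stationary.
; A one-time equip montage unlocks combat, where attacks pick random montages, nudging the index on repeats.
; Montage flags block overlapping actions, cleared by delays for dodges and a ResetAttackMontage event for attacks.
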(event `InputAxis|MouseX`
  (params (AxisValue :type "Float (single-precision)"))
  ;[1 1 1] Mouse
  (`self.AddControllerYawInput` AxisValue))

(event `self.ReceiveTick`
  (params (DeltaSeconds :type "Float (single-precision)"))
  ;[1 1 1] Tick
  (if (> (`KismetMathLibrary.VSize` (`self.GetVelocity`)) 0.0)
    (set `CharacterMovementComponent.bOrientRotationToMovement` false (`self.CharacterMovement`))
    (else
      (set `CharacterMovementComponent.bOrientRotationToMovement` true (`self.CharacterMovement`)))))

(event `InputAxis|MouseY`
  (params (AxisValue :type "Float (single-precision)"))
  ;[1 1 1] Mouse
  (`self.AddControllerPitchInput` AxisValue))

(event `InputAxis|MoveForward`
  (params (AxisValue :type "Float (single-precision)"))
  ;[1 1 1] Move
  (`self.AddMovementInput` (`KismetMathLibrary.GetForwardVector` (`KismetMathLibrary.MakeRotator` 0.0 0.0 (.yaw (`self.GetControlRotation`)))) AxisValue))

(event `Key|One`
  (params (Key :type "Key Structure"))
  ;[1 1 1] Equip
  (:`Pressed`
    (`/Engine/EditorBlueprintResources/StandardMacros.DoOnce` false
      (:`Completed`
        ;;[1 1 1] Equip Animation Montage Length is 2.6sec
        (`AnimInstance.Montage_Play` (`SkeletalMeshComponent.GetAnimInstance` (`self.Mesh`)) "/Game/GhostSamurai_Katana/GhostSamurai_Katana/Animation/Common/Root/GhostSamurai_APose_Equip02_Root_Montage.GhostSamurai_APose_Equip02_Root_Montage" 1.0 "MontageLength" 0.0 true)
        (`KismetSystemLibrary.Delay` 2.5)
        (set `self.Equip` true)))))

(event `InputAxis|MoveRight`
  (params (AxisValue :type "Float (single-precision)"))
  ;[1 1 1] Move
  (`self.AddMovementInput` (`KismetMathLibrary.GetRightVector` (`KismetMathLibrary.MakeRotator` 0.0 0.0 (.yaw (`self.GetControlRotation`)))) AxisValue))

(event `InputAction|Run`
  (params (Key :type "Key Structure"))
  ;[1 1 1] Basic Action
  (:`Pressed`
    (if (not (`self.Defense`))
      (set `self.Run` true)
      (bind (_direction _runvalue) (`Timeline|RunTimeLine` :!label _label)
        (:`Update`
          (set `CharacterMovementComponent.MaxWalkSpeed` _runvalue (`self.CharacterMovement`))))))
  (:`Released`
    (set `self.Run` false :!label _label_2)
    (goto _label :!via `Reverse`)))

(event `InputAction|Attack`
  (params (Key :type "Key Structure"))
  (bind _attack_num (`self.Attack Num`))
  (:`Pressed`
    (if (`self.Equip`)
      (if (not (or (`self.DodgeMontagePlay`) (`self.AttackMontage`)))
        (set `self.AttackMontage` true)
        (bind _output_get (set `self.Attack Num` (`KismetMathLibrary.RandomIntegerInRange` 0 4)))
        (if (== _output_get (`self.Curr Attacck Num`))
          (if (== _attack_num 0)
            (bind _result (`/Engine/EditorBlueprintResources/StandardMacros.IncrementInt` _attack_num)
              (:`  `
                (set `self.Curr Attacck Num` _result)))
            (else
              (bind _result_2 (`/Engine/EditorBlueprintResources/StandardMacros.DecrementInt` _attack_num)
                (:`  `
                  (set `self.Curr Attacck Num` _result_2)))))
          (else
            (set `self.Curr Attacck Num` _output_get)))
        (`AnimInstance.Montage_Play` (`SkeletalMeshComponent.GetAnimInstance` (`self.Mesh`)) (`|GetArrayItem` (`self.Attack Montage to Play`) (`self.Curr Attacck Num`)) 1.2 "MontageLength" 0.0 true)))))

(event `InputAction|Defense`
  (params (Key :type "Key Structure"))
  ;[1 1 1] Basic Action
  (:`Pressed`
    (if (`self.Run`)
      (`|ExecutionSequence`
        (:`then_0`
          (goto _label_2))
        (:`then_1`
          _)))
    (set `self.Defense` true))
  (:`Released`
    (set `self.Defense` false)))

(event `Reset Attack Montage`
  (set `self.AttackMontage` false))

(event `InputAction|Dodge`
  (params (Key :type "Key Structure"))
  (bind _returnvalue (`self.GetInputAxisValue`))
  (bind _returnvalue_2 (`self.GetInputAxisValue`))
  (bind _returnvalue_3 (`SkeletalMeshComponent.GetAnimInstance` (`self.Mesh`)))
  (bind _returnvalue_4 (`SkeletalMeshComponent.GetAnimInstance` (`self.Mesh`)))
  ;[1 1 1] Dodge
  (:`Pressed`
    (if (`self.Equip`)
      (if (not (or (`self.DodgeMontagePlay`) (`self.AttackMontage`)))
        (set `self.DodgeMontagePlay` true)
        (if (!= _returnvalue_2 0.0)
          (if (> _returnvalue_2 0.0)
            ;;[1 1 1] Front / Back Dodge
            (`AnimInstance.Montage_Play` _returnvalue_4 "/Game/GhostSamurai_Katana/GhostSamurai_Katana/Animation/Apose/Dodge/Root/GhostSamurai_APose_Dodge_F_Root_Montage.GhostSamurai_APose_Dodge_F_Root_Montage" 1.2 "MontageLength" 0.0 true)
            (else
              (`AnimInstance.Montage_Play` _returnvalue_4 "/Game/GhostSamurai_Katana/GhostSamurai_Katana/Animation/Apose/Dodge/Root/GhostSamurai_APose_Dodge_B_Root_Montage.GhostSamurai_APose_Dodge_B_Root_Montage" 1.2 "MontageLength" 0.0 true :!label _label_3)))
          (`KismetSystemLibrary.Delay` 1.0)
          (set `self.DodgeMontagePlay` false)
          (elif (!= _returnvalue 0.0)
            (if (> _returnvalue 0.0)
              ;;[1 1 1] Right / Left Dodge
              (`AnimInstance.Montage_Play` _returnvalue_3 "/Game/GhostSamurai_Katana/GhostSamurai_Katana/Animation/Apose/Dodge/Root/GhostSamurai_APose_Dodge_R_Root_Montage.GhostSamurai_APose_Dodge_R_Root_Montage" 1.2 "MontageLength" 0.0 true)
              (else
                (`AnimInstance.Montage_Play` _returnvalue_3 "/Game/GhostSamurai_Katana/GhostSamurai_Katana/Animation/Apose/Dodge/Root/GhostSamurai_APose_Dodge_L_Root_Montage.GhostSamurai_APose_Dodge_L_Root_Montage" 1.2 "MontageLength" 0.0 true)))
            (`KismetSystemLibrary.Delay` 0.6)
            (set `self.DodgeMontagePlay` false)
            (else
              (goto _label_3))))))))

(fn `UserConstructionScript`)